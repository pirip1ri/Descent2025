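; BP_Sensor is a one-shot sensor that raises the alarm when it detects the player.
; Its DetectPlayer event checks the passed actor for the Player tag, latches HasDetected, plays a camera shutter sound and starts the BP_Alarm found by class lookup.
; It also plays a point light timeline that sets intensity to zero on every update, as the Lerp meant to scale intensity is unconnected.
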(event `Detect Player`
  (params (`Actor Detected` :type "Actor Object Reference"))
  (if (and (`self.ActorHasTag` `Actor Detected` "Player") (not (`self.Has Detected`)))
    (set `self.Has Detected` true)
    (`GameplayStatics.PlaySoundAtLocation` "/Engine/VREditor/Sounds/UI/Camera_Shutter.Camera_Shutter" (`self.K2_GetActorLocation`) (struct) 1.0 1.0 0.0 "/Game/AI/Audio/Alarms/SA_Sensor.SA_Sensor" null null null)
    (bind _returnvalue (`GameplayStatics.GetActorOfClass` "/Game/AI/Sensors_Alarms/BP_Alarm.BP_Alarm_C"))
    (`/Game/AI/Sensors_Alarms/BP_Alarm.Start Alarm` _returnvalue)
    (bind (_direction _intensity_of_light) (`Timeline|Point Light Timeline`)
      (:`Update`
        (`LightComponent.SetIntensity` (`self.PointLight`) 0.0)))))

(fn `UserConstructionScript`)