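; BP_Alarm is an alarm actor that raises a global alert when triggered.
; StartAlarm spawns the alarm sound at its location, guarded by an active flag, and StopAlarm fades it out.
; Starting it also sets HasSeenPlayer on every BP_Guard's blackboard through its AI controller and tells the Descent game mode to switch to escape music.
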(event `Start Alarm`
  ;[1 1 1] Start Alarm
  (if (not (`self.Alarm Active`))
    (bind _returnvalue (`GameplayStatics.SpawnSoundAtLocation` "/Game/AI/Audio/Alarms/MS_Alarm.MS_Alarm" (`self.K2_GetActorLocation`) (struct) 1.0 1.0 0.0 null null))
    (set `self.Alarm Sound` _returnvalue)
    (set `self.Alarm Active` true)
    (`self.AlertGuards`)))

(event `Stop Alarm`
  ;[1 1 1] Stop Alarm
  (if (`self.Alarm Active`)
    (`AudioComponent.FadeOut` (`self.Alarm Sound`) 1.0 0.0 "Linear")
    (set `self.Alarm Active` false)))

(event `AlertGuards`
  ;[1 1 1] Alert Guards/Music Escape
  (bind _outactors (`GameplayStatics.GetAllActorsOfClass` "/Game/AI/Enemy/BP_Guard.BP_Guard_C"))
  (for _array_element _outactors
    (bind _asbpi_ai_enemy (cast `/Game/AI/Enemy/BPI_AI_Enemy` (`AIBlueprintHelperLibrary.GetAIController` _array_element)))
    (`BlackboardComponent.SetValueAsBool` (`AIBlueprintHelperLibrary.GetBlackboard` _asbpi_ai_enemy) "HasSeenPlayer" true))
  (bind _asbp_descent_game_mode_base (cast `/Game/GameMode/BP_DescentGameModeBase` (`GameplayStatics.GetGameMode`)))
  (`/Game/GameMode/BP_DescentGameModeBase.SwitchMusicToEscape` _asbp_descent_game_mode_base))

(event `self.ReceiveBeginPlay`)

(fn `UserConstructionScript`)