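; Rotating AI alarm sensor whose head continuously sweeps back and forth through a half turn.
; On BeginPlay, the Motion timeline interpolates the Head's relative rotation, and a FlipFlop on completion alternates reverse and forward playback.
; DetectPlayer is called when an actor ends overlap with TriggerDetectionZone, rather than on entering it.
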(event `self.TriggerDetectionZone.OnComponentEndOverlap`
  (params (OverlappedComponent :type "PrimitiveComponent Object Reference") (OtherActor :type "Actor Object Reference") (OtherComp :type "PrimitiveComponent Object Reference") (OtherBodyIndex :type Integer))
  (`self.Detect Player` OtherActor))

(event `self.ReceiveBeginPlay`
  (bind (_direction _rotation) (`Timeline|Motion` :!label _label)
    (:`Update`
      (`SceneComponent.K2_SetRelativeRotation` (`self.Head`) (`KismetMathLibrary.RLerp` (struct :`Yaw` 90.0) (struct :`Yaw` -90.0) _rotation) false false))
    (:`Finished`
      (`/Engine/EditorBlueprintResources/StandardMacros.FlipFlop`
        (:`A`
          (goto _label :!via `Reverse`))
        (:`B`
          (goto _label))))))

(fn `UserConstructionScript`
  (`parent.UserConstructionScript`))