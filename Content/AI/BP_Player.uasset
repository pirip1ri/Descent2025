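; Player Blueprint that handles movement, camera look and interaction through Enhanced Input, adding its mapping context on BeginPlay.
; Move input is applied relative to control rotation yaw, and look input drives controller yaw and inverted pitch.
; Interact sends an interface message to every overlapping actor that implements BPI_Interact, with no trace or single-target selection.
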(event `EnhancedInput|/Game/AI/Input/IA_Interact`
  (params (ActionValue :type Boolean) (ElapsedSeconds :type "Float (double-precision)") (TriggeredSeconds :type "Float (double-precision)") (InputAction :type "InputAction Object Reference" :default "/Game/AI/Input/IA_Interact.IA_Interact"))
  (:`Started`
    (for _array_element (`self.GetOverlappingActors` null)
      (if (`KismetSystemLibrary.DoesImplementInterface` _array_element "/Game/AI/BPI_Interact.BPI_Interact_C")
        (message `/Game/AI/BPI_Interact.Interact` _array_element)))))

(event `self.ReceiveBeginPlay`
  (`EnhancedInputSubsystemInterface.AddMappingContext` (pcsubsystem `EnhancedInputLocalPlayerSubsystem` (`GameplayStatics.GetPlayerController` 0)) "/Game/AI/Input/IMC_PlayerInput.IMC_PlayerInput" 0 (struct)))

(event `EnhancedInput|/Game/AI/Input/IA_Move`
  (params (ActionValue :type "Vector2D Structure") (ElapsedSeconds :type "Float (double-precision)") (TriggeredSeconds :type "Float (double-precision)") (InputAction :type "InputAction Object Reference" :default "/Game/AI/Input/IA_Move.IA_Move"))
  (bind (_returnvalue_roll _returnvalue_pitch _returnvalue_yaw) (`KismetMathLibrary.BreakRotator` (`self.GetControlRotation`)))
  (bind (_returnvalue_roll_2 _returnvalue_pitch_2 _returnvalue_yaw_2) (`KismetMathLibrary.BreakRotator` (`self.GetControlRotation`)))
  (:`Triggered`
    (`self.AddMovementInput` (`KismetMathLibrary.GetRightVector` (`KismetMathLibrary.MakeRotator` _returnvalue_roll 0.0 _returnvalue_yaw)) ActionValue_X)
    (`self.AddMovementInput` (`KismetMathLibrary.GetForwardVector` (`KismetMathLibrary.MakeRotator` 0.0 0.0 _returnvalue_yaw_2)) ActionValue_Y)))

(event `EnhancedInput|/Game/AI/Input/IA_Look`
  (params (ActionValue :type "Vector2D Structure") (ElapsedSeconds :type "Float (double-precision)") (TriggeredSeconds :type "Float (double-precision)") (InputAction :type "InputAction Object Reference" :default "/Game/AI/Input/IA_Look.IA_Look"))
  (:`Triggered`
    (`self.AddControllerYawInput` ActionValue_X)
    (`self.AddControllerPitchInput` (* ActionValue_Y -1.0))))

(fn `UserConstructionScript`)