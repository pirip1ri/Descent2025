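; BP_TestDoor is an interactable test door that swings open and closed.
; Its InteractAbility event forwards to InteractAbilityCall, while OpenDoor and CloseDoor set the door state and play or reverse one timeline driving the mesh's yaw.
; The shared Finished handler resolves Opening to Opened or Closing to Closed, and disables the interaction sphere's collision once the door is open.
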(event `self.InteractAbility`
  (`self.InteractAbilityCall`))

(event `self.OpenDoor`
  (`self.SetDoorState` "Opening")
  (bind (_direction _rotation_value) (`Timeline|Door Opening Timeline` :!label _label)
    (:`Update`
      (`SceneComponent.K2_SetRelativeRotation` (`self.DoorMesh`) (`KismetMathLibrary.MakeRotator` 0.0 0.0 _rotation_value) false false))
    (:`Finished`
      (bind _returnvalue (`self.GetDoorState`))
      (switch `EDoorState` _returnvalue
        (:`Opening`
          (`self.SetDoorState` "Opened")
          (`PrimitiveComponent.SetCollisionEnabled` (`self.InteractionSphere`) "NoCollision"))
        (:`Closing`
          (`self.SetDoorState` "Closed"))))))

(event `self.CloseDoor`
  (`self.SetDoorState` "Closing")
  (goto _label :!via `Reverse`))

(fn `UserConstructionScript`)