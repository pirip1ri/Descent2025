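; BP_TestDoor is a test door prop that swings open and closed through yaw rotation of its static mesh.
; OpenDoor and CloseDoor play and reverse a shared timeline, whose finish handler resolves the Opening or Closing state to Opened or Closed.
; Reaching Opened disables InteractionBox collision, and nothing here re-enables it.
; InteractAbility forwards to InteractAbilityCall, while overlapping InteractionBox only prints a debug string.
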(event `self.InteractAbility`
  (`self.InteractAbilityCall`))

(event `self.OpenDoor`
  (`self.SetDoorState` "Opening")
  (bind (_direction _rotation_value) (`Timeline|Door Opening Timeline` :!label _label)
    (:`Update`
      (`SceneComponent.K2_SetRelativeRotation` (`self.StaticMesh`) (`KismetMathLibrary.MakeRotator` 0.0 0.0 _rotation_value) false false))
    (:`Finished`
      (bind _returnvalue (`self.GetDoorState`))
      (switch `EDoorState` _returnvalue
        (:`Opening`
          (`self.SetDoorState` "Opened")
          (`PrimitiveComponent.SetCollisionEnabled` (`self.InteractionBox`) "NoCollision"))
        (:`Closing`
          (`self.SetDoorState` "Closed"))))))

(event `self.CloseDoor`
  (`self.SetDoorState` "Closing")
  (goto _label :!via `Reverse`))

(event `self.InteractionBox.OnComponentBeginOverlap`
  (params (OverlappedComponent :type "PrimitiveComponent Object Reference") (OtherActor :type "Actor Object Reference") (OtherComp :type "PrimitiveComponent Object Reference") (OtherBodyIndex :type Integer) (bFromSweep :type Boolean) (SweepResult :type "HitResult Structure (by ref)"))
  (`KismetSystemLibrary.PrintString` "Hello"))

(fn `UserConstructionScript`)